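; Player controller for a chat feature, handling name entry and message submission for the player.
; On BeginPlay the local controller shows the name-entry widget and mouse cursor.
; Entering a name forwards it to BP_Gamemode through SubmitName, then swaps the name widget for the message widget.
; Chat entries reach the game mode through OnSubmitMsg, with both paths passing player controller 0 as the sender.
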(event Custom|SubmitName
  (params (PlayerController :type BP%20Player%20Controller%20Object%20Reference) (NewName :type String))
  (bind _asbp_gamemode (Utilities|Casting|CastToBP_Gamemode (Game|GetGameMode)))
  (Default|OnChangeName _asbp_gamemode PlayerController NewName))

(event Custom|OnEnterName
  (params (NewName :type String))
  (bind _asbp_player_controller (Utilities|Casting|CastToBP_PlayerController (Game|GetPlayerController 0)))
  (CallFunction|SubmitName _asbp_player_controller NewName)
  (bind _foundwidgets (Widget|GetAllWidgetsOfClass "/Game/Widgets/Widget_NameUI.Widget_NameUI_C" true))
  (Widget|RemovefromParent _foundwidgets)
  (bind _returnvalue (UserInterface|CreateWidget "/Game/Widgets/Widget_MsgUI.Widget_MsgUI_C"))
  (UserInterface|Viewport|AddtoViewport _returnvalue 0))

(event Custom|OnEnterChat
  (params (Msg :type String))
  (bind _asbp_player_controller (Utilities|Casting|CastToBP_PlayerController (Game|GetPlayerController 0)))
  (CallFunction|OnSubmitMsg _asbp_player_controller Msg))

(event Custom|OnSubmitMsg
  (params (PlayerController :type BP%20Player%20Controller%20Object%20Reference) (Msg :type String))
  (bind _asbp_gamemode (Utilities|Casting|CastToBP_Gamemode (Game|GetGameMode)))
  (Default|OnReceivedMsg _asbp_gamemode PlayerController Msg))

(event EventBeginPlay
  (if (Pawn|IsLocalPlayerController)
    (bind _returnvalue (UserInterface|CreateWidget "/Game/Widgets/Widget_NameUI.Widget_NameUI_C"))
    (UserInterface|Viewport|AddtoViewport _returnvalue 0)
    (Variables|Default|SetbShowMouseCursor true)))

(event EventTick
  (params (DeltaSeconds :type Float%20%28single-precision%29)))

(fn ConstructionScript)